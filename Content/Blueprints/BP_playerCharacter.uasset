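; First-person player character with movement, mouse look, footstep audio, interaction and physics pickup.
; Short camera traces scale the HUD crosshair over interactables, send interface messages on left click and grab physics-handle objects with E, which follow PhysRoot each tick.
; ToggleCrosshair switches between interactive play and cursor mode by flipping the Interactive gate and HUD visibility; right click restores play.
; Tick polls movement axes to play pitch-randomized footsteps.
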(event EventTick
  (params (DeltaSeconds :type Float%20%28single-precision%29))
  (bind _footstep (Variables|Default|GetFootStep))
  (bind _fpcamera (Variables|Default|GetFPCamera))
  (bind _returnvalue (Transformation|GetWorldLocation _fpcamera))
  ;[1 1 1] Tick
  (Utilities|FlowControl|Sequence
    (:then_0
      ;[1 1 1] Adjust held object call
      (if (Variables|Default|GetIsHolding)
        (CallFunction|PhysHeldAdjust)))
    (:then_1
      ;[1 1 1] FootStep SFX
      (Math|Float|CompareFloat (Input|AxisValues|GetinputAxis_MoveForward) 0.0
        (:>
          (if (not (Audio|Components|Audio|IsPlaying _footstep)) :!label _label
            (Math|Integer|CompareInt (Variables|Default|GetStepCycle) 0
              (:>
                _)
              (:==
                (Utilities|FlowControl|Delay 0.2)))
            (Audio|Components|Audio|SetPitchMultiplier _footstep (Math|Random|RandomFloatinRange 0.85 0.98))
            (Audio|Components|Audio|Play _footstep 0.0)
            (Variables|Default|SetStepCycle 1)))
        (:==
          (Math|Float|CompareFloat (Input|AxisValues|GetinputAxis_StrafeLeft) 0.0
            (:>
              (goto _label))
            (:==
              (Variables|Default|SetStepCycle 0))
            (:<
              (goto _label))))
        (:<
          (goto _label))))
    (:then_2
      ;[1 1 1] Look function
      (bind (_outhit _returnvalue_2) (Collision|LineTraceByChannel _returnvalue (+ (* (Math|Vector|GetForwardVector _fpcamera) 2e+02) _returnvalue) "TraceTypeQuery2" true 0 "None"))
      (if _returnvalue_2
        (if (Utilities|DoesObjectImplementInterface (.HitActor (Collision|BreakHitResult _outhit)) "/Game/Blueprints/Interfaces/BPI_interactionInterface.BPI_interactionInterface_C")
          (bind _scalevector (Timeline|chScaleTimeline Play)
            (:Update
              (bind _output_get (Variables|Default|SetchScaleRef (Math|Conversions|ToVector2D(Vector) _scalevector)))
              (Default|PlayerLook (Variables|Default|GetHUD_reference) _output_get)))
          (else
            (Timeline|chScaleTimeline Reverse)))
        (else
          (Timeline|chScaleTimeline Reverse))))))

(event EventBeginPlay
  ;[1 1 1] HUD_Setup
  (bind _returnvalue (UserInterface|CreateWidget "/Game/Blueprints/UI/WID_HUD.WID_HUD_C" 0 1.0))
  (bind _output_get (Variables|Default|SetHUD_reference _returnvalue))
  (UserInterface|Viewport|AddtoViewport _output_get 0))

(event EventToggleCrosshair
  (bind _returnvalue (Game|GetPlayerController 0))
  (bind _hud_reference (Variables|Default|GetHUD_reference))
  ;[1 1 1] Toggle crosshair and interactivity
  (if (Variables|Default|GetCrosshairDrawn)
    (Widget|SetVisibility _hud_reference "Hidden")
    (Variables|Default|SetCrosshairDrawn false)
    (Variables|Default|SetInteractive false)
    (Variables|/Script/Engine.PlayerController|SetbShowMouseCursor _returnvalue true)
    (Variables|/Script/Engine.PlayerController|SetbEnableMouseOverEvents _returnvalue true)
    (else
      (Widget|SetVisibility _hud_reference "Visible")
      (Variables|Default|SetCrosshairDrawn true)
      (Variables|Default|SetInteractive true)
      (Variables|/Script/Engine.PlayerController|SetbShowMouseCursor _returnvalue false)
      (Variables|/Script/Engine.PlayerController|SetbEnableMouseOverEvents _returnvalue false))))

(event Input|AxisEvents|InputAxisinputAxis_Pitch
  (params (AxisValue :type Float%20%28single-precision%29))
  ;[1 1 1] Mouse_Look_Input
  (if (Variables|Default|GetInteractive)
    (Pawn|Input|AddControllerPitchInput AxisValue)))

(event Input|AxisEvents|InputAxisinputAxis_MoveForward
  (params (AxisValue :type Float%20%28single-precision%29))
  ;[1 1 1] Keyboard_Movement_Input
  (if (Variables|Default|GetInteractive)
    (Pawn|Input|AddMovementInput (Math|Vector|GetForwardVector (Math|Rotator|MakeRotator 0.0 0.0 (.Yaw (Math|Rotator|BreakRotator (Pawn|GetControlRotation :!class /Script/Engine.Pawn))))) (* AxisValue (Variables|Default|Getspeed_Scale)) false)))

(event Input|AxisEvents|InputAxisinputAxis_StrafeLeft
  (params (AxisValue :type Float%20%28single-precision%29))
  ;[1 1 1] Keyboard_Movement_Input
  (if (Variables|Default|GetInteractive)
    (Pawn|Input|AddMovementInput (Math|Vector|GetRightVector (Math|Rotator|MakeRotator 0.0 0.0 (.Yaw (Math|Rotator|BreakRotator (Pawn|GetControlRotation :!class /Script/Engine.Pawn))))) (* AxisValue (Variables|Default|Getspeed_Scale)) false)))

(event Input|AxisEvents|InputAxisinputAxis_Yaw
  (params (AxisValue :type Float%20%28single-precision%29))
  ;[1 1 1] Mouse_Look_Input
  (if (Variables|Default|GetInteractive)
    (Pawn|Input|AddControllerYawInput AxisValue)))

(event Input|MouseEvents|LeftMouseButton
  (params (Key :type Key%20Structure :default "AnyKey"))
  (bind _fpcamera (Variables|Default|GetFPCamera))
  (bind _returnvalue (Transformation|GetWorldLocation _fpcamera))
  ;[1 1 1] Interaction
  (:Pressed
    (if (Variables|Default|GetInteractive)
      (bind (_outhit _returnvalue_2) (Collision|LineTraceByChannel _returnvalue (+ (* (Math|Vector|GetForwardVector _fpcamera) 2e+02) _returnvalue) "TraceTypeQuery2" true 0 "None"))
      (if _returnvalue_2
        (if (Utilities|DoesObjectImplementInterface (.HitActor (Collision|BreakHitResult _outhit)) "/Game/Blueprints/Interfaces/BPI_interactionInterface.BPI_interactionInterface_C")
          (Class|BPIInteractionInterface|PlayerInteract(Message) (.HitActor (Collision|BreakHitResult _outhit)) self))))))

(event Input|KeyboardEvents|E
  (params (Key :type Key%20Structure :default "AnyKey"))
  (bind _fpcamera (Variables|Default|GetFPCamera))
  (bind _returnvalue (Transformation|GetWorldLocation _fpcamera))
  (:Pressed
    (if (Variables|Default|GetIsHolding)
      (Physics|Components|PhysicsHandle|ReleaseComponent (Variables|Default|GetPickupPhysHandle))
      (Variables|Default|SetIsHolding false)
      (elif (Variables|Default|GetInteractive)
        (bind (_outhit _returnvalue_2) (Collision|LineTraceByChannel _returnvalue (+ (* (Math|Vector|GetForwardVector _fpcamera) 2e+02) _returnvalue) "TraceTypeQuery2" true 0 "None"))
        (if _returnvalue_2
          (if (Utilities|DoesObjectImplementInterface (.HitActor (Collision|BreakHitResult _outhit)) "/Game/Blueprints/Interfaces/BPI_PhysicsHandleInterface.BPI_PhysicsHandleInterface_C")
            (Class|PhysicsHandleComponent|GrabComponent (Variables|Default|GetPickupPhysHandle) (.HitComponent (Collision|BreakHitResult _outhit)) "None" (Transformation|GetWorldLocation (.HitComponent (Collision|BreakHitResult _outhit))) false)
            (Variables|Default|SetIsHolding true)))))))

(event Input|MouseEvents|RightMouseButton
  (params (Key :type Key%20Structure :default "AnyKey"))
  ;[1 1 1] Console eject
  (:Pressed
    (if (not (Variables|Default|GetInteractive))
      (Input|SetInputModeGameOnly (Game|GetPlayerController 0))
      (CallFunction|ToggleCrosshair))))

(fn ConstructionScript)

(fn PhysHeldAdjust
  (Physics|Components|PhysicsHandle|SetTargetLocation (Variables|Default|GetPickupPhysHandle) (Transformation|GetWorldLocation (Variables|Default|GetPhysRoot))))