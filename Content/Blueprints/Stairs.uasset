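; Stairs is a construction-script Blueprint that builds a staircase from repeated instances of an InstancedStaticMesh.
; The step count is the rounded ratio of EndPoint's length to Offset's length.
; A loop places each unrotated, unit-scale instance at a multiple of Offset, so EndPoint sets only the run's length, while Offset sets its direction and spacing.
; The event graph has no active logic.
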(event EventBeginPlay)

(event EventActorBeginOverlap
  (params (OtherActor :type Actor%20Object%20Reference)))

(event EventTick
  (params (DeltaSeconds :type Float%20%28single-precision%29)))

(fn ConstructionScript
  (bind _endpoint (Variables|Default|GetEndPoint))
  (bind _offset (Variables|Default|GetOffset))
  (bind _returnvalue (Math|Vector|VectorLength _endpoint))
  (bind _returnvalue_2 (Math|Vector|VectorLength _offset))
  (bind _returnvalue_3 (/ _returnvalue _returnvalue_2))
  (bind _returnvalue_4 (Math|Float|Round _returnvalue_3))
  (if (> _returnvalue_4 0)
    (for _index (range 0 _returnvalue_4)
      (Components|InstancedStaticMesh|AddInstance (Variables|Default|GetInstancedStaticMesh) (Math|Transform|MakeTransform (* _offset _index) "0, 0, 0" "1,1,1")))))