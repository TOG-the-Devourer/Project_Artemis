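; BP_testGamemode is a game mode that silences level ambience on the main menu and tracks whether all three parts are held.
; On BeginPlay, if the level is Main_Menu, it casts player character 0 to BP_playerCharacter and stops its LevelAmbience.
; Tick polls the HaveBoots, HaveGoggles and HaveChest flags and sets AllParts once all are true; nothing here clears it.
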(event EventTick
  (params (DeltaSeconds :type Float%20%28single-precision%29))
  (if (Variables|Default|GethaveBoots)
    (if (Variables|Default|GethaveGoggles)
      (if (Variables|Default|GethaveChest)
        (Variables|Default|SetAllParts true)))))

(event EventBeginPlay
  (bind _returnvalue (Game|GetCurrentLevelName true))
  (if (Utilities|Enum|Equal(Enum) _returnvalue "Main_Menu")
    (bind _asbp_player_character (Utilities|Casting|CastToBP_playerCharacter (Game|GetPlayerCharacter 0)))
    (Audio|Components|Audio|Stop (Variables|/Game/Blueprints/BP_playerCharacter.BP_playerCharacter_C|GetLevelAmbience _asbp_player_character))))

(fn ConstructionScript)