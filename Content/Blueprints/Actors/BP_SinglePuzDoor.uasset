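; A puzzle door that destroys itself on player interaction once its cannon-press sequence is solved.
; CannonPress checks each pressed cannon's index against the expected one for the current step, changing its material on a match and marking the puzzle complete when the step counter check reaches three.
; A wrong press switches all four cannons to a fail material, resets progress and ignores presses during a brief delay before restoring them.
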(event EventPlayerInteract
  (params (playerRef :type BP%20Player%20Character%20Object%20Reference))
  ;[1 1 1] Interaction
  (if (Variables|Default|GetPuzComplete)
    (Actor|DestroyActor)))

(event EventCannonPress
  (params (CanInd :type Integer) (CurrentCan :type BP%20Single%20Cannon%20Test%20Object%20Reference))
  (if (not (Variables|Default|GetFailed))
    (Variables|Default|SetCurrentCan CurrentCan)
    (Variables|Default|SetCanInd CanInd)
    (Variables|Default|SetMatInd 1)
    (switch int (Variables|Default|GetPressIndex)
      (:0
        (Math|Integer|CompareInt (Variables|Default|GetCanInd) (Variables|Default|GetFirstCan)
          (:>
            (Variables|Default|SetMatInd 2 :!label _label)
            (Variables|Default|SetFailed true)
            (Utilities|FlowControl|Sequence
              (:then_0
                (Default|SetMaterial (Variables|Default|GetCan1) (Variables|Default|GetMatInd)))
              (:then_1
                (Default|SetMaterial (Variables|Default|GetCan2) (Variables|Default|GetMatInd)))
              (:then_2
                (Default|SetMaterial (Variables|Default|GetCan3) (Variables|Default|GetMatInd)))
              (:then_3
                (Default|SetMaterial (Variables|Default|GetCan4) (Variables|Default|GetMatInd))
                (Variables|Default|SetPressIndex 0)
                (Utilities|FlowControl|Delay 0.9)
                (Variables|Default|SetFailed false)
                (Variables|Default|SetMatInd 0)
                (Utilities|FlowControl|Sequence
                  (:then_0
                    (Default|SetMaterial (Variables|Default|GetCan1) (Variables|Default|GetMatInd)))
                  (:then_1
                    (Default|SetMaterial (Variables|Default|GetCan2) (Variables|Default|GetMatInd)))
                  (:then_2
                    (Default|SetMaterial (Variables|Default|GetCan3) (Variables|Default|GetMatInd)))
                  (:then_3
                    (Default|SetMaterial (Variables|Default|GetCan4) (Variables|Default|GetMatInd)))))))
          (:==
            (Default|SetMaterial (Variables|Default|GetCurrentCan) (Variables|Default|GetMatInd))
            (bind _result (Math|Integer|IncrementInt (Variables|Default|GetPressIndex) :!label _label_2)
              (:%20%20
                (Math|Integer|CompareInt _result 3
                  (:==
                    (Variables|Default|SetPuzComplete true))))))
          (:<
            (goto _label))))
      (:1
        (Math|Integer|CompareInt (Variables|Default|GetCanInd) (Variables|Default|GetSecondCan)
          (:>
            (goto _label))
          (:==
            (Default|SetMaterial (Variables|Default|GetCurrentCan) (Variables|Default|GetMatInd))
            (goto _label_2))
          (:<
            (goto _label))))
      (:2
        (Math|Integer|CompareInt (Variables|Default|GetCanInd) (Variables|Default|GetThirdCan)
          (:>
            (goto _label))
          (:==
            (Default|SetMaterial (Variables|Default|GetCurrentCan) (Variables|Default|GetMatInd))
            (goto _label_2))
          (:<
            (goto _label))))
      (:3
        (Math|Integer|CompareInt (Variables|Default|GetCanInd) (Variables|Default|GetFourthCan)
          (:>
            (goto _label))
          (:==
            (Default|SetMaterial (Variables|Default|GetCurrentCan) (Variables|Default|GetMatInd))
            (goto _label_2))
          (:<
            (goto _label)))))))

(fn ConstructionScript)