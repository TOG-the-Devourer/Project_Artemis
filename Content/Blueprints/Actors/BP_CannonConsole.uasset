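; BP_CannonConsole is an in-world console with a widget screen that rotates its parent cannon as part of a puzzle.
; BeginPlay creates the WID_CannonConsole screen, and PuzzleSetup links it and a sequencer to the console and cannon.
; Rot toggles a rotating flag, and Tick turns the parent by a fixed per-frame step in either direction.
; PlayerInteract toggles the player's crosshair.
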(event EventTick
  (params (DeltaSeconds :type Float%20%28single-precision%29))
  (bind _parentref (Variables|Default|GetParentRef))
  (if (Variables|Default|GetIsRotating)
    (switch int (stale EventRot RotDirection)
      (:0
        (Class|Actor|AddActorWorldRotation _parentref "0,-1.000000, 0"))
      (:1
        (Class|Actor|AddActorWorldRotation _parentref "0,1.000000, 0")))))

(event EventBeginPlay
  (bind _conwid (Variables|Default|GetConWid))
  (Utilities|FlowControl|Sequence
    (:then_0
      (Class|WidgetComponent|SetDrawSize _conwid "(X=1920.000000,Y=1080.000000)")
      (bind _returnvalue (UserInterface|CreateWidget "/Game/Blueprints/Widgets/WID_CannonConsole.WID_CannonConsole_C"))
      (bind _output_get (Variables|Default|SetWIDRef _returnvalue))
      (UserInterface|SetWidget _conwid _output_get)
      (Class|WidgetComponent|SetMaxInteractionDistance _conwid 2e+02))))

(event EventRot
  (params (Rot :type Boolean) (RotDirection :type Integer))
  (if Rot
    (Variables|Default|SetIsRotating true)
    (else
      (Variables|Default|SetIsRotating false))))

(event EventPuzzleSetup
  (params (ParentRef :type BP%20Cannon%20Master%20Object%20Reference))
  (bind _self self)
  (bind _output_get (Variables|Default|SetParentRef ParentRef))
  (Default|ConsoleSetup (Variables|Default|GetWIDRef) _self _output_get)
  (Default|SequencerSetup (Variables|Default|GetSeqRef) _self _output_get))

(event EventPlayerInteract
  (params (playerRef :type BP%20Player%20Character%20Object%20Reference))
  (Default|ToggleCrosshair playerRef))

(fn ConstructionScript)