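; Master cannon actor for what appears to be a button-driven puzzle, tracking which valid target the cannon points at.
; On BeginPlay it passes itself to its linked MyBut through PuzzleSetup.
; Each Tick it line-traces forward from CastOrigin, ignoring the player and four button references.
; A hit actor implementing BPI_CannonInterface has its object name stored in TargName, which is otherwise cleared.
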(event EventTick
  (params (DeltaSeconds :type Float%20%28single-precision%29))
  (bind _castorigin (Variables|Default|GetCastOrigin))
  (bind _returnvalue (Transformation|GetWorldLocation _castorigin))
  (bind (_outhit _returnvalue_2) (Collision|LineTraceByChannel _returnvalue (+ _returnvalue (* (Math|Vector|GetForwardVector _castorigin) 1.5e+03)) "TraceTypeQuery1" false (Utilities|Array|MakeArray (Game|GetPlayerCharacter 0) (Variables|Default|GetBut1) (Variables|Default|GetBut2) (Variables|Default|GetBut3) (Variables|Default|GetBut4)) "None"))
  (if _returnvalue_2
    (if (Utilities|DoesObjectImplementInterface (.HitActor (Collision|BreakHitResult _outhit)) "/Game/Blueprints/Interfaces/BPI_CannonInterface.BPI_CannonInterface_C")
      (Variables|Default|SetTargName (Utilities|GetObjectName (.HitActor (Collision|BreakHitResult _outhit))))
      (else
        (Variables|Default|SetTargName "" :!label _label)))
    (else
      (goto _label))))

(event EventBeginPlay
  (Default|PuzzleSetup (Variables|Default|GetMyBut) self))

(fn ConstructionScript)