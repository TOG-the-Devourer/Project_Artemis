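; Exit door that opens when a Character enters its box and closes when one leaves, gated by the AllParts flag copied from BP_testGamemode at BeginPlay.
; A DoorMovement timeline plays or reverses, offsetting both door halves and the base from cached relative transforms.
; IsPlaying blocks triggers mid-motion, so the door rechecks player overlap after each move to correct its state.
; Overlap-triggered moves play open/close sounds scaled by the player's FSFXVolume.
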(event OnComponentEndOverlap(Box)
  (params (OtherActor :type Actor%20Object%20Reference) (OtherComp :type Primitive%20Component%20Object%20Reference) (OtherBodyIndex :type Integer))
  (bind _audio (Variables|Default|GetAudio))
  (bind _doorleft (Variables|Default|GetDoorLeft))
  (bind _doorright (Variables|Default|GetDoorRight))
  (bind _doorbase (Variables|Default|GetDoorBase))
  (if (Variables|Default|GetAllParts)
    (Utilities|Casting|CastToCharacter OtherActor)
    (if (not (Variables|Default|GetIsPlaying))
      (Variables|Default|SetIsPlaying true)
      (Math|Integer|CompareInt (Variables|Default|GetActIndex) 0
        (:==
          (Variables|Default|SetActIndex 1)
          (Utilities|FlowControl|Sequence
            (:then_0
              (Math|Integer|CompareInt (Variables|Default|GetActIndex) 0
                (:>
                  (bind (_direction _doorleft_2 _doorright_2 _doorbase_2) (Timeline|DoorMovement ReverseFromEnd)
                    (:Update
                      (Utilities|FlowControl|Sequence
                        (:then_0
                          (Transformation|SetRelativeLocation (Variables|Default|GetDoorLeft) (+ (.location (Math|Transform|MakeTransform (Math|Vector|MakeVector (.X (Math|Vector|BreakVector _doorleft_2)) 0.0 (.Y (Math|Vector|BreakVector _doorleft_2))) (.Rotation (Math|Transform|BreakTransform (Transformation|GetRelativeTransform _doorleft))) (Transformation|GetWorldScale _doorleft))) (.location (Variables|Default|GetDoorLeftTran))) false false))
                        (:then_1
                          (Transformation|SetRelativeTransform (Variables|Default|GetDoorRight) (Math|Transform|MakeTransform (+ (.location (Math|Transform|MakeTransform (Math|Vector|MakeVector (.X (Math|Vector|BreakVector _doorright_2)) 0.0 (.Y (Math|Vector|BreakVector _doorright_2))) (.Rotation (Math|Transform|BreakTransform (Transformation|GetRelativeTransform _doorright))) (Transformation|GetWorldScale _doorright))) (.location (Variables|Default|GetDoorRightTran))) (.rotation (Math|Transform|MakeTransform (Math|Vector|MakeVector (.X (Math|Vector|BreakVector _doorright_2)) 0.0 (.Y (Math|Vector|BreakVector _doorright_2))) (.Rotation (Math|Transform|BreakTransform (Transformation|GetRelativeTransform _doorright))) (Transformation|GetWorldScale _doorright))) (.scale (Math|Transform|MakeTransform (Math|Vector|MakeVector (.X (Math|Vector|BreakVector _doorright_2)) 0.0 (.Y (Math|Vector|BreakVector _doorright_2))) (.Rotation (Math|Transform|BreakTransform (Transformation|GetRelativeTransform _doorright))) (Transformation|GetWorldScale _doorright)))) false false))
                        (:then_2
                          (Transformation|SetRelativeTransform (Variables|Default|GetDoorBase) (Math|Transform|MakeTransform (+ (.location (Math|Transform|MakeTransform (Math|Vector|MakeVector 0.0 0.0 (.X (Math|Vector|BreakVector _doorbase_2))) (.Rotation (Math|Transform|BreakTransform (Transformation|GetRelativeTransform _doorbase))) (Transformation|GetWorldScale _doorbase))) (.location (Variables|Default|GetDoorBaseTran))) (.rotation (Math|Transform|MakeTransform (Math|Vector|MakeVector 0.0 0.0 (.X (Math|Vector|BreakVector _doorbase_2))) (.Rotation (Math|Transform|BreakTransform (Transformation|GetRelativeTransform _doorbase))) (Transformation|GetWorldScale _doorbase))) (.scale (Math|Transform|MakeTransform (Math|Vector|MakeVector 0.0 0.0 (.X (Math|Vector|BreakVector _doorbase_2))) (.Rotation (Math|Transform|BreakTransform (Transformation|GetRelativeTransform _doorbase))) (Transformation|GetWorldScale _doorbase)))) false false))))
                    (:Finished
                      (Utilities|FlowControl|Delay 0.3)
                      (Variables|Default|SetIsPlaying false)
                      (Math|Integer|CompareInt (Variables|Default|GetActIndex) 1
                        (:==
                          (Variables|Default|SetOpen false))
                        (:<
                          (Variables|Default|SetOpen true)))
                      (if (Collision|IsOverlappingActor (Variables|Default|GetBox) (Game|GetPlayerCharacter 0) :!class /Script/Engine.PrimitiveComponent) :!label _label
                        (if (not (Variables|Default|GetOpen))
                          (if (Variables|Default|GetIsPlaying)
                            (goto _label)
                            (else
                              (Variables|Default|SetActIndex 0)
                              (Variables|Default|SetOpen true)
                              (Timeline|DoorMovement Play))))
                        (elif (Variables|Default|GetOpen)
                          (if (Variables|Default|GetIsPlaying)
                            (goto _label)
                            (else
                              (Variables|Default|SetActIndex 1)
                              (Variables|Default|SetOpen false)
                              (Timeline|DoorMovement ReverseFromEnd))))))))
                (:==
                  (Timeline|DoorMovement Play))))
            (:then_1
              (Audio|Components|Audio|SetVolumeMultiplier _audio (* (Variables|/Game/Blueprints/BP_playerCharacter.BP_playerCharacter_C|GetF_SFX_Volume (Variables|Default|Get1pCharRef)) 0.16) :!class /Script/Engine.AudioComponent)
              (Math|Integer|CompareInt (Variables|Default|GetActIndex) 0
                (:>
                  (Audio|Components|Audio|SetSound _audio "/Game/Audio/SFX/DoorClose.DoorClose")
                  (Audio|Components|Audio|Play _audio 0.0))
                (:==
                  (Audio|Components|Audio|SetSound _audio "/Game/Audio/SFX/DoorOpen.DoorOpen")
                  (Audio|Components|Audio|Play _audio 0.0))))))))))

(event OnComponentBeginOverlap(Box)
  (params (OtherActor :type Actor%20Object%20Reference) (OtherComp :type Primitive%20Component%20Object%20Reference) (OtherBodyIndex :type Integer) (bFromSweep :type Boolean) (SweepResult :type Hit%20Result%20Structure%20%28by%20ref%29))
  (bind _audio (Variables|Default|GetAudio))
  (bind _doorleft (Variables|Default|GetDoorLeft))
  (bind _doorright (Variables|Default|GetDoorRight))
  (bind _doorbase (Variables|Default|GetDoorBase))
  (if (Variables|Default|GetAllParts)
    (Utilities|Casting|CastToCharacter OtherActor)
    (if (not (Variables|Default|GetIsPlaying))
      (Variables|Default|SetIsPlaying true)
      (Math|Integer|CompareInt (Variables|Default|GetActIndex) 1
        (:==
          (Variables|Default|SetActIndex 0)
          (Utilities|FlowControl|Sequence
            (:then_0
              (Math|Integer|CompareInt (Variables|Default|GetActIndex) 0
                (:>
                  (bind (_direction _doorleft_2 _doorright_2 _doorbase_2) (Timeline|DoorMovement ReverseFromEnd)
                    (:Update
                      (Utilities|FlowControl|Sequence
                        (:then_0
                          (Transformation|SetRelativeLocation (Variables|Default|GetDoorLeft) (+ (.location (Math|Transform|MakeTransform (Math|Vector|MakeVector (.X (Math|Vector|BreakVector _doorleft_2)) 0.0 (.Y (Math|Vector|BreakVector _doorleft_2))) (.Rotation (Math|Transform|BreakTransform (Transformation|GetRelativeTransform _doorleft))) (Transformation|GetWorldScale _doorleft))) (.location (Variables|Default|GetDoorLeftTran))) false false))
                        (:then_1
                          (Transformation|SetRelativeTransform (Variables|Default|GetDoorRight) (Math|Transform|MakeTransform (+ (.location (Math|Transform|MakeTransform (Math|Vector|MakeVector (.X (Math|Vector|BreakVector _doorright_2)) 0.0 (.Y (Math|Vector|BreakVector _doorright_2))) (.Rotation (Math|Transform|BreakTransform (Transformation|GetRelativeTransform _doorright))) (Transformation|GetWorldScale _doorright))) (.location (Variables|Default|GetDoorRightTran))) (.rotation (Math|Transform|MakeTransform (Math|Vector|MakeVector (.X (Math|Vector|BreakVector _doorright_2)) 0.0 (.Y (Math|Vector|BreakVector _doorright_2))) (.Rotation (Math|Transform|BreakTransform (Transformation|GetRelativeTransform _doorright))) (Transformation|GetWorldScale _doorright))) (.scale (Math|Transform|MakeTransform (Math|Vector|MakeVector (.X (Math|Vector|BreakVector _doorright_2)) 0.0 (.Y (Math|Vector|BreakVector _doorright_2))) (.Rotation (Math|Transform|BreakTransform (Transformation|GetRelativeTransform _doorright))) (Transformation|GetWorldScale _doorright)))) false false))
                        (:then_2
                          (Transformation|SetRelativeTransform (Variables|Default|GetDoorBase) (Math|Transform|MakeTransform (+ (.location (Math|Transform|MakeTransform (Math|Vector|MakeVector 0.0 0.0 (.X (Math|Vector|BreakVector _doorbase_2))) (.Rotation (Math|Transform|BreakTransform (Transformation|GetRelativeTransform _doorbase))) (Transformation|GetWorldScale _doorbase))) (.location (Variables|Default|GetDoorBaseTran))) (.rotation (Math|Transform|MakeTransform (Math|Vector|MakeVector 0.0 0.0 (.X (Math|Vector|BreakVector _doorbase_2))) (.Rotation (Math|Transform|BreakTransform (Transformation|GetRelativeTransform _doorbase))) (Transformation|GetWorldScale _doorbase))) (.scale (Math|Transform|MakeTransform (Math|Vector|MakeVector 0.0 0.0 (.X (Math|Vector|BreakVector _doorbase_2))) (.Rotation (Math|Transform|BreakTransform (Transformation|GetRelativeTransform _doorbase))) (Transformation|GetWorldScale _doorbase)))) false false))))
                    (:Finished
                      (Utilities|FlowControl|Delay 0.3)
                      (Variables|Default|SetIsPlaying false)
                      (Math|Integer|CompareInt (Variables|Default|GetActIndex) 1
                        (:==
                          (Variables|Default|SetOpen false))
                        (:<
                          (Variables|Default|SetOpen true)))
                      (if (Collision|IsOverlappingActor (Variables|Default|GetBox) (Game|GetPlayerCharacter 0) :!class /Script/Engine.PrimitiveComponent) :!label _label
                        (if (not (Variables|Default|GetOpen))
                          (if (Variables|Default|GetIsPlaying)
                            (goto _label)
                            (else
                              (Variables|Default|SetActIndex 0)
                              (Variables|Default|SetOpen true)
                              (Timeline|DoorMovement Play))))
                        (elif (Variables|Default|GetOpen)
                          (if (Variables|Default|GetIsPlaying)
                            (goto _label)
                            (else
                              (Variables|Default|SetActIndex 1)
                              (Variables|Default|SetOpen false)
                              (Timeline|DoorMovement ReverseFromEnd))))))))
                (:==
                  (Timeline|DoorMovement Play))))
            (:then_1
              (Audio|Components|Audio|SetVolumeMultiplier _audio (* (Variables|/Game/Blueprints/BP_playerCharacter.BP_playerCharacter_C|GetF_SFX_Volume (Variables|Default|Get1pCharRef)) 0.16) :!class /Script/Engine.AudioComponent)
              (Math|Integer|CompareInt (Variables|Default|GetActIndex) 0
                (:>
                  (Audio|Components|Audio|SetSound _audio "/Game/Audio/SFX/DoorClose.DoorClose")
                  (Audio|Components|Audio|Play _audio 0.0))
                (:==
                  (Audio|Components|Audio|SetSound _audio "/Game/Audio/SFX/DoorOpen.DoorOpen")
                  (Audio|Components|Audio|Play _audio 0.0))))))))))

(event EventBeginPlay
  (Utilities|FlowControl|Sequence
    (:then_0
      (Components|Timeline|SetPlayRate (Variables|Default|GetDoorMovement) 1.05)
      (bind _asbp_player_character (Utilities|Casting|CastToBP_playerCharacter (Game|GetPlayerCharacter 0)))
      (Variables|Default|Set1pCharRef _asbp_player_character))
    (:then_1
      (Variables|Default|SetDoorLeftTran (Transformation|GetRelativeTransform (Variables|Default|GetDoorLeft)))
      (Variables|Default|SetDoorRightTran (Transformation|GetRelativeTransform (Variables|Default|GetDoorRight)))
      (Variables|Default|SetDoorBaseTran (Transformation|GetRelativeTransform (Variables|Default|GetDoorBase))))
    (:then_2
      (bind _asbp_test_gamemode (Utilities|Casting|CastToBP_testGamemode (Game|GetGameMode)))
      (bind _output_get (Variables|Default|SetNewVar_0 _asbp_test_gamemode))
      (Variables|Default|SetAllParts (Variables|/Game/Blueprints/BP_testGamemode.BP_testGamemode_C|GetAllParts _output_get)))))

(fn ConstructionScript)