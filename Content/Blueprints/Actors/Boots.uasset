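; Boots is an interactable pickup actor that represents boots the player can collect.
; On PlayerInteract it plays a sound, shows the legs slot on the player's HUD and passes its item name to BP_playerCharacter.
; It then hides both meshes and disables their collision, shows an inventory notification widget for two seconds, and destroys itself.
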(event EventBeginPlay)

(event EventActorBeginOverlap
  (params (OtherActor :type Actor%20Object%20Reference)))

(event EventTick
  (params (DeltaSeconds :type Float%20%28single-precision%29)))

(event EventPlayerInteract
  (params (playerRef :type BP%20Player%20Character%20Object%20Reference))
  (bind _staticmesh (Variables|Default|GetStaticMesh))
  (Audio|PlaySound2D "/Game/Audio/SFX/Test_SFX/sound-select-electronic.sound-select-electronic")
  (Variables|/Game/Blueprints/UI/WID_HUD.WID_HUD_C|SetW_LEGS_VISIBILITY (Variables|/Game/Blueprints/BP_playerCharacter.BP_playerCharacter_C|GetHUD_reference playerRef) "Visible")
  (bind _asbp_player_character (Utilities|Casting|CastToBP_playerCharacter (Game|GetPlayerCharacter 0)))
  (Variables|/Game/Blueprints/BP_playerCharacter.BP_playerCharacter_C|SetpickedUpItemName _asbp_player_character (.ItemName (Utilities|Struct|BreakS_ItemData (Variables|Default|GetS_ItemData))))
  (bind _returnvalue (UserInterface|CreateWidget "/Game/Blueprints/Widgets/InventoryWidget/W_INV_Notificaiton.W_INV_Notificaiton_C"))
  (UserInterface|Viewport|AddtoViewport _returnvalue 0)
  (Rendering|SetVisibility _staticmesh false false)
  (Collision|SetCollisionEnabled _staticmesh "NoCollision")
  (Utilities|FlowControl|Delay 2.0)
  (Widget|RemovefromParent _returnvalue)
  (Actor|DestroyActor))

(fn ConstructionScript)