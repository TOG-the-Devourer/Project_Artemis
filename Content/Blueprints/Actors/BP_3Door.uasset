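; Three-part automatic door that opens when a Character enters its trigger Box and closes when one leaves.
; The DoorMovement timeline offsets left and right panels in X and Z and the base in Z, relative to transforms cached at BeginPlay.
; IsPlaying blocks retriggering mid-animation and ActIndex tracks direction.
; When opening finishes, the timeline reverses if the player character is no longer inside the Box.
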(event OnComponentEndOverlap(Box)
  (params (OtherActor :type Actor%20Object%20Reference) (OtherComp :type Primitive%20Component%20Object%20Reference) (OtherBodyIndex :type Integer))
  (Utilities|Casting|CastToCharacter OtherActor)
  (if (not (Variables|Default|GetIsPlaying))
    (Variables|Default|SetIsPlaying true)
    (Math|Integer|CompareInt (Variables|Default|GetActIndex) 0
      (:==
        (Variables|Default|SetActIndex 1)
        (bind (_direction _doorleft _doorright _doorbase) (Timeline|DoorMovement ReverseFromEnd)
          (:Update
            (Utilities|FlowControl|Sequence
              (:then_0
                (Transformation|SetRelativeLocation (Variables|Default|GetDoorLeft) (+ (.location (Math|Transform|MakeTransform (Math|Vector|MakeVector (.X (Math|Vector|BreakVector _doorleft)) 0.0 (.Y (Math|Vector|BreakVector _doorleft))) "0, 0, 0" (Transformation|GetWorldScale (Variables|Default|GetDoorLeft)))) (.location (Variables|Default|GetDoorLeftTran))) false false))
              (:then_1
                (Transformation|SetRelativeTransform (Variables|Default|GetDoorRight) (Math|Transform|MakeTransform (+ (.location (Math|Transform|MakeTransform (Math|Vector|MakeVector (.X (Math|Vector|BreakVector _doorright)) 0.0 (.Y (Math|Vector|BreakVector _doorright))) "0, 0, 0" (Transformation|GetWorldScale (Variables|Default|GetDoorRight)))) (.location (Variables|Default|GetDoorRightTran))) "0, 0, 0" (.scale (Math|Transform|MakeTransform (Math|Vector|MakeVector (.X (Math|Vector|BreakVector _doorright)) 0.0 (.Y (Math|Vector|BreakVector _doorright))) "0, 0, 0" (Transformation|GetWorldScale (Variables|Default|GetDoorRight))))) false false))
              (:then_2
                (Transformation|SetRelativeTransform (Variables|Default|GetDoorBase) (Math|Transform|MakeTransform (+ (.location (Math|Transform|MakeTransform (Math|Vector|MakeVector 0.0 0.0 (.X (Math|Vector|BreakVector _doorbase))) "0, 0, 0" (Transformation|GetWorldScale (Variables|Default|GetDoorBase)))) (.location (Variables|Default|GetDoorBaseTran))) "0, 0, 0" (.scale (Math|Transform|MakeTransform (Math|Vector|MakeVector 0.0 0.0 (.X (Math|Vector|BreakVector _doorbase))) "0, 0, 0" (Transformation|GetWorldScale (Variables|Default|GetDoorBase))))) false false))))
          (:Finished
            (Variables|Default|SetIsPlaying false)
            (Math|Integer|CompareInt (Variables|Default|GetActIndex) 1
              (:==
                (Variables|Default|SetOpen false))
              (:<
                (Variables|Default|SetOpen true)))
            (if (not (Collision|IsOverlappingActor (Variables|Default|GetBox) (Game|GetPlayerCharacter 0) :!class /Script/Engine.PrimitiveComponent))
              (if (Variables|Default|GetOpen)
                (Variables|Default|SetActIndex 1)
                (Variables|Default|SetOpen false)
                (Timeline|DoorMovement ReverseFromEnd)))))))))

(event OnComponentBeginOverlap(Box)
  (params (OtherActor :type Actor%20Object%20Reference) (OtherComp :type Primitive%20Component%20Object%20Reference) (OtherBodyIndex :type Integer) (bFromSweep :type Boolean) (SweepResult :type Hit%20Result%20Structure%20%28by%20ref%29))
  (Utilities|Casting|CastToCharacter OtherActor)
  (if (not (Variables|Default|GetIsPlaying))
    (Variables|Default|SetIsPlaying true)
    (Math|Integer|CompareInt (Variables|Default|GetActIndex) 1
      (:==
        (Variables|Default|SetActIndex 0)
        (bind (_direction _doorleft _doorright _doorbase) (Timeline|DoorMovement Play)
          (:Update
            (Utilities|FlowControl|Sequence
              (:then_0
                (Transformation|SetRelativeLocation (Variables|Default|GetDoorLeft) (+ (.location (Math|Transform|MakeTransform (Math|Vector|MakeVector (.X (Math|Vector|BreakVector _doorleft)) 0.0 (.Y (Math|Vector|BreakVector _doorleft))) "0, 0, 0" (Transformation|GetWorldScale (Variables|Default|GetDoorLeft)))) (.location (Variables|Default|GetDoorLeftTran))) false false))
              (:then_1
                (Transformation|SetRelativeTransform (Variables|Default|GetDoorRight) (Math|Transform|MakeTransform (+ (.location (Math|Transform|MakeTransform (Math|Vector|MakeVector (.X (Math|Vector|BreakVector _doorright)) 0.0 (.Y (Math|Vector|BreakVector _doorright))) "0, 0, 0" (Transformation|GetWorldScale (Variables|Default|GetDoorRight)))) (.location (Variables|Default|GetDoorRightTran))) "0, 0, 0" (.scale (Math|Transform|MakeTransform (Math|Vector|MakeVector (.X (Math|Vector|BreakVector _doorright)) 0.0 (.Y (Math|Vector|BreakVector _doorright))) "0, 0, 0" (Transformation|GetWorldScale (Variables|Default|GetDoorRight))))) false false))
              (:then_2
                (Transformation|SetRelativeTransform (Variables|Default|GetDoorBase) (Math|Transform|MakeTransform (+ (.location (Math|Transform|MakeTransform (Math|Vector|MakeVector 0.0 0.0 (.X (Math|Vector|BreakVector _doorbase))) "0, 0, 0" (Transformation|GetWorldScale (Variables|Default|GetDoorBase)))) (.location (Variables|Default|GetDoorBaseTran))) "0, 0, 0" (.scale (Math|Transform|MakeTransform (Math|Vector|MakeVector 0.0 0.0 (.X (Math|Vector|BreakVector _doorbase))) "0, 0, 0" (Transformation|GetWorldScale (Variables|Default|GetDoorBase))))) false false))))
          (:Finished
            (Variables|Default|SetIsPlaying false)
            (Math|Integer|CompareInt (Variables|Default|GetActIndex) 1
              (:==
                (Variables|Default|SetOpen false))
              (:<
                (Variables|Default|SetOpen true)))
            (if (not (Collision|IsOverlappingActor (Variables|Default|GetBox) (Game|GetPlayerCharacter 0) :!class /Script/Engine.PrimitiveComponent))
              (if (Variables|Default|GetOpen)
                (Variables|Default|SetActIndex 1)
                (Variables|Default|SetOpen false)
                (Timeline|DoorMovement ReverseFromEnd)))))))))

(event EventBeginPlay
  (Variables|Default|SetDoorLeftTran (Transformation|GetRelativeTransform (Variables|Default|GetDoorLeft)))
  (Variables|Default|SetDoorRightTran (Transformation|GetRelativeTransform (Variables|Default|GetDoorRight)))
  (Variables|Default|SetDoorBaseTran (Transformation|GetRelativeTransform (Variables|Default|GetDoorBase))))

(fn ConstructionScript)