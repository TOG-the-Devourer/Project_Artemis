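; Puzzle door actor that the player can remove by interacting once a four-cannon sequence puzzle is solved, destroying itself.
; PuzzleSetup stores references to four separate cannon classes by index.
; PressCannon checks presses against a hardcoded order through a step counter, switching each correct cannon's material and setting PuzSolved after the last.
; A wrong press shows a fail material on all cannons, resets progress and briefly blocks input before restoring their default material.
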(event EventPressCannon
  (params (cannonIndex :type Integer) (cannon :type Actor%20Object%20Reference))
  ;[1 1 1] Sequence Check
  (if (not (Variables|Default|Getfailed))
    (switch int (Variables|Default|GetpressIndex)
      (:0
        (Math|Integer|CompareInt cannonIndex 1
          (:>
            ;[1 1 1] Fail Handling
            (Utilities|FlowControl|Sequence :!label _label
              (:then_0
                (Default|SetMat (Variables|Default|Getcannon1Ref) 2))
              (:then_1
                (Default|SetMat (Variables|Default|Getcannon2Ref) 2))
              (:then_2
                (Default|SetMat (Variables|Default|Getcannon3Ref) 2))
              (:then_3
                (Default|SetMat (Variables|Default|Getcannon4Ref) 2)))
            (Variables|Default|SetpressIndex 0)
            (Variables|Default|Setfailed true)
            (Utilities|FlowControl|Delay 1.0)
            (Variables|Default|Setfailed false)
            (Utilities|FlowControl|Sequence
              (:then_0
                (Default|SetMat (Variables|Default|Getcannon1Ref)))
              (:then_1
                (Default|SetMat (Variables|Default|Getcannon2Ref)))
              (:then_2
                (Default|SetMat (Variables|Default|Getcannon3Ref)))
              (:then_3
                (Default|SetMat (Variables|Default|Getcannon4Ref)))))
          (:==
            (Default|SetMat (Variables|Default|Getcannon2Ref) 1)
            (Math|Integer|IncrementInt (Variables|Default|GetpressIndex)))
          (:<
            (goto _label))))
      (:1
        (Math|Integer|CompareInt cannonIndex 2
          (:>
            (goto _label))
          (:==
            (Default|SetMat (Variables|Default|Getcannon3Ref) 1)
            (Math|Integer|IncrementInt (Variables|Default|GetpressIndex)))
          (:<
            (goto _label))))
      (:2
        (Math|Integer|CompareInt cannonIndex 0
          (:>
            (goto _label))
          (:==
            (Default|SetMat (Variables|Default|Getcannon1Ref) 1)
            (Math|Integer|IncrementInt (Variables|Default|GetpressIndex)))
          (:<
            (goto _label))))
      (:3
        (Math|Integer|CompareInt cannonIndex 3
          (:>
            (goto _label))
          (:==
            (Default|SetMat (Variables|Default|Getcannon4Ref) 1)
            (Math|Integer|IncrementInt (Variables|Default|GetpressIndex)
              (:%20%20
                (Variables|Default|SetpuzSolved true))))
          (:<
            (goto _label)))))))

(event EventPuzzleSetup
  (params (Cannon_ref :type Actor%20Object%20Reference) (Cannon_In :type Integer))
  ;[1 1 1] Set Cannon References
  (switch int Cannon_In
    (:0
      (bind _asbp_cannon (Utilities|Casting|CastToBP_Cannon Cannon_ref))
      (Variables|Default|Setcannon1Ref _asbp_cannon))
    (:1
      (bind _asbp_cannon_2 (Utilities|Casting|CastToBP_Cannon2 Cannon_ref))
      (Variables|Default|Setcannon2Ref _asbp_cannon_2))
    (:2
      (bind _asbp_cannon_3 (Utilities|Casting|CastToBP_Cannon3 Cannon_ref))
      (Variables|Default|Setcannon3Ref _asbp_cannon_3))
    (:3
      (bind _asbp_cannon_4 (Utilities|Casting|CastToBP_Cannon4 Cannon_ref))
      (Variables|Default|Setcannon4Ref _asbp_cannon_4))))

(event EventPlayerInteract
  (params (playerRef :type BP%20Player%20Character%20Object%20Reference))
  ;[1 1 1] Interaction
  (if (Variables|Default|GetpuzSolved)
    (Actor|DestroyActor)))

(fn ConstructionScript)