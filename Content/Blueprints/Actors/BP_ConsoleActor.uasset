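; BP_ConsoleActor is an interactable in-world console that shows a Console widget linked to a door button reference.
; On BeginPlay it adds a widget component, creates the Console widget, keeps it as PanelRef and passes ButDoorRef to its ButSetup.
; PlayerInteract toggles the player's crosshair and calls the player's Setup with the console itself, and PlayerEject toggles the crosshair again.
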(event EventPlayerInteract
  (params (playerRef :type BP%20Player%20Character%20Object%20Reference))
  (Default|ToggleCrosshair playerRef)
  (Default|Setup playerRef self))

(event EventPlayerEject
  (Default|ToggleCrosshair (stale EventPlayerInteract playerRef)))

(event EventBeginPlay
  (bind _returnvalue (AddComponent|AddWidgetComponent false))
  (bind _returnvalue_2 (UserInterface|CreateWidget "/Game/Blueprints/Widgets/Console.Console_C"))
  (bind _output_get (Variables|Default|SetPanelRef _returnvalue_2))
  (UserInterface|SetWidget _returnvalue _output_get)
  (Default|ButSetup (Variables|Default|GetPanelRef) (Variables|Default|GetButDoorRef)))

(fn ConstructionScript)