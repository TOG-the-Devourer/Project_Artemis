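; BP_Cannon3 is an interactable cannon actor that serves as one input in a cannon puzzle controlled by a linked puzzle door.
; On BeginPlay it registers itself with PuzDoor under a fixed index, and player interaction reports a press to that door.
; A SetMat event swaps the mesh material between unpressed, correct and incorrect states as feedback.
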(event EventPlayerInteract
  (params (playerRef :type BP%20Player%20Character%20Object%20Reference))
  (Default|PressCannon (Variables|Default|GetpuzDoor) 2 self))

(event EventSetMat
  (params (matIndex :type Integer))
  (bind _int (Variables|Default|GetInt))
  (switch int matIndex
    (:0
      (Rendering|Material|SetMaterial _int 0 "/Game/Materials/MAT_Unpressed.MAT_Unpressed"))
    (:1
      (Rendering|Material|SetMaterial _int 0 "/Game/Materials/MAT_Correct.MAT_Correct"))
    (:2
      (Rendering|Material|SetMaterial _int 0 "/Game/Materials/MAT_Incorrect.MAT_Incorrect"))))

(event EventBeginPlay
  (Default|PuzzleSetup (Variables|Default|GetpuzDoor) self 2))

(fn ConstructionScript)