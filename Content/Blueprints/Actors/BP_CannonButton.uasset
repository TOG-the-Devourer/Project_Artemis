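; BP_CannonButton is a puzzle button actor that reports its sequence number to a puzzle container for checking.
; On BeginPlay it creates a WID_CannonButton on an added widget component with limited interaction range, passing itself to the widget.
; A press calls SeqCheck on the container, while check results and resets are relayed to the widget.
; Player interaction toggles that player's crosshair.
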(event EventBeginPlay
  (bind _returnvalue (AddComponent|AddWidgetComponent false (Math|Transform|MakeTransform "0, 0,92.693489" "25.629904,89.998711,0.000099" "0.296631,0.296631,0.296631")))
  (bind _returnvalue_2 (UserInterface|CreateWidget "/Game/Blueprints/Widgets/WID_CannonButton.WID_CannonButton_C"))
  (bind _output_get (Variables|Default|SetButton _returnvalue_2))
  (UserInterface|SetWidget _returnvalue _output_get)
  (Class|WidgetComponent|SetMaxInteractionDistance _returnvalue 2e+02)
  (Class|BPICannonInterface|PuzzleSetup(Message) _output_get self))

(event EventButtonPressed
  (Default|SeqCheck (Variables|Default|GetPuzContainer) (Variables|Default|GetSeqInt) self))

(event EventPlayerInteract
  (params (playerRef :type BP%20Player%20Character%20Object%20Reference))
  (Default|ToggleCrosshair playerRef))

(event EventSeqCheckReturn
  (params (SeqReturn :type Boolean))
  (Default|SeqCheckReturn (Variables|Default|GetButton) SeqReturn))

(event EventReset
  (Default|Reset (Variables|Default|GetButton)))

(fn ConstructionScript)