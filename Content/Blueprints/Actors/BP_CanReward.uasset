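; BP_CanReward is a four-cannon sequence puzzle actor meant to spawn a BP_Chest_Piece at its own transform location when solved.
; SeqCheck steps PuzInd through four integer comparisons, and a mismatch calls SeqFail on all cannons, then SeqReset after a one-second delay.
; As wired, each comparison's input is a constant zero, so every check fails and the solved branch is never reached.
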(event EventSeqCheck
  (bind _self self)
  (bind _puzind (Variables|Default|GetPuzInd))
  (bind _returnvalue (Transformation|GetActorTransform _self))
  (if (not (Variables|Default|GetIsFailed))
    (Variables|Default|SetCurCan 0)
    (switch int (Variables|Default|GetPuzInd)
      (:0
        (Math|Integer|CompareInt 0 1
          (:>
            (CallFunction|SeqFail :!label _label)
            (Utilities|FlowControl|Delay 1.0)
            (CallFunction|SeqReset)
            (Variables|Default|SetIsFailed false))
          (:==
            (Math|Integer|IncrementInt _puzind
              (:%20%20
                (Default|SeqCheckReturn (Variables|Default|GetCurCan) :!label _label_2))))
          (:<
            (goto _label))))
      (:1
        (Math|Integer|CompareInt 0 2
          (:>
            (goto _label))
          (:==
            (Math|Integer|IncrementInt _puzind
              (:%20%20
                (goto _label_2))))
          (:<
            (goto _label))))
      (:2
        (Math|Integer|CompareInt 0 3
          (:>
            (goto _label))
          (:==
            (Math|Integer|IncrementInt _puzind
              (:%20%20
                (goto _label_2))))
          (:<
            (goto _label))))
      (:3
        (Math|Integer|CompareInt 0 4
          (:>
            (goto _label))
          (:==
            (Utilities|FlowControl|Sequence
              (:then_0
                (goto _label_2))
              (:then_1
                (Variables|Default|SetIsSolved true)
                (Game|SpawnActorfromClass "/Game/Blueprints/Actors/BP_Chest_Piece.BP_Chest_Piece_C" (Math|Transform|MakeTransform (.location _returnvalue) (.rotation _returnvalue) "-7.315976,-7.315976,-7.315976") "Undefined" 0 0))))
          (:<
            (goto _label)))))))

(fn ConstructionScript)

(fn SeqFail
  (Variables|Default|SetIsFailed true)
  (Utilities|FlowControl|Sequence
    (:then_0
      (Variables|Default|SetCurCan (Variables|Default|GetCannon1)))
    (:then_1
      (Variables|Default|SetCurCan (Variables|Default|GetCannon2)))
    (:then_2
      (Variables|Default|SetCurCan (Variables|Default|GetCannon3)))
    (:then_3
      (Variables|Default|SetCurCan (Variables|Default|GetCannon4))))
  (Default|SeqCheckReturn (Variables|Default|GetCurCan)))

(fn SeqReset
  (Variables|Default|SetIsFailed false)
  (Variables|Default|SetPuzInd 0)
  (Utilities|FlowControl|Sequence
    (:then_0
      (Variables|Default|SetCurCan (Variables|Default|GetCannon1)))
    (:then_1
      (Variables|Default|SetCurCan (Variables|Default|GetCannon2)))
    (:then_2
      (Variables|Default|SetCurCan (Variables|Default|GetCannon3)))
    (:then_3
      (Variables|Default|SetCurCan (Variables|Default|GetCannon4))))
  (Default|Reset (Variables|Default|GetCurCan)))

(fn SeqCheckReturn
  (return false))